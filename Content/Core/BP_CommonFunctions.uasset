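; BP_CommonFunctions provides shared helper functions for reaching game-wide state and creating battle actions.
; One helper casts the game instance to BP_GameInstance, and another reads the BattleManager stored on it.
; CreateAttackAction constructs a BP_Action_Attack object with the game instance as its Outer, assigns the given Attack and returns it.
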(fn `CreateAttackAction`
  (params (Attack :type "/Game/Blueprints/Attacks/S_Attacks Structure"))
  (returns (AttackAction :type "/Game/Blueprints/Actions/BP_Action_Attack Object Reference"))
  (bind _gameinstance (`self.GetCustomGameInstance` null))
  (bind _returnvalue (`|GenericCreateObject` "/Game/Blueprints/Actions/BP_Action_Attack.BP_Action_Attack_C" _gameinstance))
  (set `/Game/Blueprints/Actions/BP_Action_Attack.Attack` Attack _returnvalue)
  (return _returnvalue))

(fn `GetBattleManagerFromInstance`
  (returns (BattleManager :type "/Game/Blueprints/Battle/BP_BattleManager Object Reference"))
  (bind _gameinstance (`self.GetCustomGameInstance` null))
  (return (`/Game/Core/BP_GameInstance.BattleManager` _gameinstance)))

(fn `GetCustomGameInstance`
  (returns (GameInstance :type "/Game/Core/BP_GameInstance Object Reference"))
  (bind _asbp_game_instance (cast `/Game/Core/BP_GameInstance` (`GameplayStatics.GetGameInstance` null)))
  (return _asbp_game_instance))