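; Battlefield actor for Pokémon battles that serves as the player's camera view and stages the fight.
; On BeginPlay it opens the Pokémon chooser in UI-only input and registers itself with the game instance.
; InitializeBattle spawns player and enemy BP_BasePokemon at marker components, using the chosen Pokémon's material and a hardcoded Pikachu one, and adds the battle menu.
; Input handlers test saving and loading a team; an unused team-spawn branch remains.
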(event `self.ReceiveBeginPlay`
  (bind _returnvalue (`GameplayStatics.GetPlayerController` 0))
  (`PlayerController.SetViewTargetWithBlend` (`GameplayStatics.GetPlayerController` 0) self 0.0 "VTBlend_Linear" 0.0 false)
  (bind _returnvalue_2 (`|CreateWidget` "/Game/UI/WGT_PokemonChooser.WGT_PokemonChooser_C"))
  (`UserWidget.AddToViewport` _returnvalue_2 0)
  (`WidgetBlueprintLibrary.SetInputMode_UIOnlyEx` _returnvalue _returnvalue_2)
  (set `PlayerController.bShowMouseCursor` true _returnvalue)
  (bind _asbp_game_instance (cast `/Game/Core/BP_GameInstance` (`GameplayStatics.GetGameInstance`)))
  (set `/Game/Core/BP_GameInstance.Battlefield` self _asbp_game_instance))

(event `InitializeBattle`
  (`|ExecutionSequence`
    (:`then_0`
      (bind _returnvalue (`|SpawnActorFromClass` "/Game/Core/Characters/BP_BasePokemon.BP_BasePokemon_C" (`SceneComponent.K2_GetComponentToWorld` (`self.PlayerMiddle`)) "Undefined" "OverrideRootScale" null null))
      (bind _gameinstance (`/Game/Core/BP_CommonFunctions.GetCustomGameInstance`))
      (`/Game/Core/Characters/BP_BasePokemon.Initialize` _returnvalue (`.Material_19_6107D57745A31AF61AFA8AB6F95F642F` (break `/Game/Characters/Pokemon/S_Pokemon` (`/Game/Characters/Pokemon/BP_PokemonData.Pokemon` (`/Game/Core/BP_GameInstance.PlayerPokemon` _gameinstance))))))
    (:`then_1`
      (bind _returnvalue_2 (`|CreateWidget` "/Game/UI/BattleMenu/WGT_BattleMenu.WGT_BattleMenu_C"))
      (`UserWidget.AddToViewport` _returnvalue_2 0))
    (:`then_2`
      (bind _returnvalue_3 (`|SpawnActorFromClass` "/Game/Core/Characters/BP_BasePokemon.BP_BasePokemon_C" (`SceneComponent.K2_GetComponentToWorld` (`self.EnemyMiddle`)) "Undefined" "OverrideRootScale" null null))
      (`/Game/Core/Characters/BP_BasePokemon.Initialize` _returnvalue_3 "/Game/Materials/M_Pikachu.M_Pikachu"))))

(event `InputAction|SaveGame`
  (params (Key :type "Key Structure"))
  (:`Pressed`
    (`KismetSystemLibrary.PrintString` "Start Saving")
    (bind _returnvalue (`GameplayStatics.CreateSaveGameObject` "/Game/Core/SaveGame/BP_SaveGame.BP_SaveGame_C"))
    (bind _returnvalue_2 (`|GenericCreateObject` "/Game/Core/BP_TeamPokemon.BP_TeamPokemon_C" self))
    (set `/Game/Core/BP_TeamPokemon.FirstPokemon` (`self.TestPokemon`) _returnvalue_2)
    (set `/Game/Core/SaveGame/BP_SaveGame.TeamPokemon` _returnvalue_2 _returnvalue)
    (`GameplayStatics.SaveGameToSlot` _returnvalue (`/Game/Core/SaveGame/BP_SaveGame.SaveSlotName` _returnvalue) (`/Game/Core/SaveGame/BP_SaveGame.UserIndex` _returnvalue))))

(event `Key|U`
  (params (Key :type "Key Structure"))
  (:`Pressed`
    (`KismetSystemLibrary.PrintString` "Start Loading")
    (bind _returnvalue (`GameplayStatics.LoadGameFromSlot` "SaveSlot1"))
    (bind _asbp_save_game (cast `/Game/Core/SaveGame/BP_SaveGame` _returnvalue))
    (`KismetSystemLibrary.PrintString` (`KismetStringLibrary.Conv_IntToString` (`KismetArrayLibrary.Array_Length` (`/Game/Core/Characters/BP_BasePokemon.AttackList` (`/Game/Core/BP_TeamPokemon.FirstPokemon` (`/Game/Core/SaveGame/BP_SaveGame.TeamPokemon` _asbp_save_game))))))))

(fn `UserConstructionScript`)