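; Battle logic helper owned by BP_Battlefield that opens the Pokemon chooser, builds a random enemy team from DT_Pokemon and creates the battle menu.
; Queued actions are split into switch and attack lists; a turn runs switches first, then plays SortedAttacks with a timed dialog before each.
; SortAttacksBySpeed fills that list by insertion, ranking attacks on priority weighted above the user's Speed.
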(event `Initialize`
  (bind _returnvalue (`GameplayStatics.GetPlayerController` 0))
  (bind _returnvalue_2 (`|CreateWidget` "/Game/UI/WGT_PokemonChooser.WGT_PokemonChooser_C"))
  (bind _output_get (set `self.PokemonChooserMenu` _returnvalue_2))
  (`/Game/UI/WGT_PokemonChooser.Initialize` _output_get self)
  (`UserWidget.AddToViewport` _output_get 0)
  (`WidgetBlueprintLibrary.SetInputMode_UIOnlyEx` _returnvalue _returnvalue_2)
  (set `PlayerController.bShowMouseCursor` true _returnvalue))

(event `InitializeBattleMenu`
  (params (UserTeam :type "Array of /Game/Characters/Pokemon/BP_PokemonData Object Reference"))
  (`|ExecutionSequence`
    (:`then_0`
      (bind _output_get (set `self.UserTeam` UserTeam))
      (set `self.ActivePlayerPokemon` (`|GetArrayItem` _output_get))
      (`self.CreateRandomEnemyPokemon`)
      (bind _output_get_2 (set `self.ActiveEnemyPokemon` (`|GetArrayItem` (`self.EnemyTeam`))))
      (bind _asbp_battlefield (cast `/Game/Blueprints/Battle/BP_Battlefield` (`self.GetOwner`)))
      (`/Game/Blueprints/Battle/BP_Battlefield.SetEnemyPokemonMaterial` _asbp_battlefield (`.Material_19_6107D57745A31AF61AFA8AB6F95F642F` (break `/Game/Characters/Pokemon/S_Pokemon` (`/Game/Characters/Pokemon/BP_PokemonData.Pokemon` _output_get_2)))))
    (:`then_1`
      (bind _returnvalue (`|CreateWidget` "/Game/UI/BattleMenu/WGT_BattleMenu.WGT_BattleMenu_C"))
      (bind _output_get_3 (set `self.BattleMenu` _returnvalue))
      (`UserWidget.AddToViewport` _output_get_3 0)
      (`/Game/UI/BattleMenu/WGT_BattleMenu.Initialize` _output_get_3 self (`self.ActivePlayerPokemon`) (`self.ActiveEnemyPokemon`)))))

(event `AddActionToList`
  (params (Action :type "/Game/Blueprints/Actions/BP_Action Object Reference"))
  (bind _asbp_action_attack (cast `/Game/Blueprints/Actions/BP_Action_Attack` Action)
    (:`then`
      (`KismetArrayLibrary.Array_Add` (`self.AttackActions`) _asbp_action_attack))
    (:`CastFailed`
      (bind _asbp_action_switch_pokemon (cast `/Game/Blueprints/Actions/BP_Action_SwitchPokemon` Action))
      (`KismetArrayLibrary.Array_Add` (`self.SwitchingActions`) _asbp_action_switch_pokemon))))

(event `StartTurn`
  (for _array_element (`self.SwitchingActions`)
    (`/Game/Blueprints/Actions/BP_Action.Execute` _array_element))
  (for _array_element_2 (`self.SortedAttacks`)
    (`/Game/UI/BattleMenu/WGT_BattleMenu.OnShowActionDialog` (`self.BattleMenu`) (`/Game/Blueprints/Actions/BP_Action_Attack.UserPokemon` _array_element_2) _array_element_2)
    (`KismetSystemLibrary.Delay` 2.0)
    (`/Game/UI/BattleMenu/WGT_BattleMenu.OnShowBattleMenu` (`self.BattleMenu`))
    (`/Game/Blueprints/Actions/BP_Action.Execute` _array_element_2)))

(fn `CalculatePriorityCount`
  (params (Attack :type "/Game/Blueprints/Actions/BP_Action_Attack Object Reference"))
  (returns (PriorityCount :type Integer))
  (return (+ (* (`.Priority_20_D7B490D54BB9973B4B3F3CBA4965E38E` (break `/Game/Blueprints/Attacks/S_Attacks` (`/Game/Blueprints/Actions/BP_Action_Attack.Attack` Attack))) 10000) (`.Speed_12_B3FF00B14BC845FC4567908E88E2E235` (break `/Game/Core/Characters/S_Stats` (`/Game/Characters/Pokemon/BP_PokemonData.CurrentStats` (`/Game/Blueprints/Actions/BP_Action_Attack.UserPokemon` Attack)))))))

(fn `CreateRandomEnemyPokemon`
  (`/Engine/EditorBlueprintResources/StandardMacros.Do N` (`KismetArrayLibrary.Array_Length` (`self.UserTeam`))
    (:`Exit`
      (bind _outrownames (`DataTableFunctionLibrary.GetDataTableRowNames` "/Game/Characters/Pokemon/DT_Pokemon.DT_Pokemon"))
      (bind _returnvalue (`|GetDataTableRow` "/Game/Characters/Pokemon/DT_Pokemon.DT_Pokemon" (`|GetArrayItem` _outrownames (`KismetMathLibrary.RandomInteger` (`KismetArrayLibrary.Array_Length` _outrownames))))
        (:`then`
          (bind _attacks (`/Game/Core/BP_PokemonDataHelper.GetAttackListByPokemon` _returnvalue))
          (bind _data (`/Game/Core/BP_PokemonDataHelper.CreatePokemonData` _returnvalue _attacks))
          (`KismetArrayLibrary.Array_Add` (`self.EnemyTeam`) _data))))))

(fn `GetActivePokemon`
  (params (bIsPlayerPokemon :type Boolean))
  (returns (Pokemon :type "/Game/Characters/Pokemon/BP_PokemonData Object Reference"))
  (if bIsPlayerPokemon
    (return (`self.ActivePlayerPokemon`))
    (else
      (return (`self.ActiveEnemyPokemon`)))))

(fn `SortAttacksBySpeed`
  (locals (bIsInsertedIntoArray :type Boolean))
  (for _array_element (`self.AttackActions`)
    (if (== (`KismetArrayLibrary.Array_Length` (`self.SortedAttacks`)) 0)
      (`KismetArrayLibrary.Array_Add` (`self.SortedAttacks`) _array_element)
      (else
        (for (_array_element_2 _array_index) (`self.SortedAttacks`)
          (bind _prioritycount (`self.CalculatePriorityCount` _array_element_2))
          (bind _prioritycount_2 (`self.CalculatePriorityCount` _array_element))
          (`/Engine/EditorBlueprintResources/StandardMacros.CompareInt` _prioritycount _prioritycount_2
            (:`==`
              (if (not (== (`KismetMathLibrary.RandomInteger` 1) 0))
                (`KismetArrayLibrary.Array_Insert` (`self.SortedAttacks`) _array_element _array_index :!label _label)
                (set `local.bIsInsertedIntoArray` true)
                (break)))
            (:`<`
              (goto _label))))
        (if (not (`local.bIsInsertedIntoArray`))
          (`KismetArrayLibrary.Array_Add` (`self.SortedAttacks`) _array_element)
          (set `local.bIsInsertedIntoArray` false))))))