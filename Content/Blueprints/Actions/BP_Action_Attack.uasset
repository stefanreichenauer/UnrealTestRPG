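; BP_Action_Attack is a battle action that makes a user Pokemon perform an attack on a target.
; InitAttackAction stores the attack, user and target; Execute rolls against the attack's accuracy and only prints a message on a miss.
; On a hit, physical or special stat pairs feed DamageCalculation, and the result goes to the target's DealDamage.
; DamageCalculation follows a Pokemon-style formula using level, power, stat ratio and modifier variables, truncating intermediate steps.
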(event `InitAttackAction`
  (params (Attack :type "/Game/Blueprints/Attacks/S_Attacks Structure") (User :type "/Game/Characters/Pokemon/BP_PokemonData Object Reference") (Target :type "/Game/Characters/Pokemon/BP_PokemonData Object Reference"))
  (set `self.Attack` Attack)
  (set `self.UserPokemon` User)
  (set `self.Target` Target))

(event `self.Execute`
  (bind _target (`self.Target`))
  (bind _target_2 (`self.Target`))
  (bind (_attackname _attacktype _type _power _accuracy) (break `/Game/Blueprints/Attacks/S_Attacks` (`self.Attack`)))
  (bind ((`Attack_8_D6E035E0481ED0BD9F67F28671794986` _attack) (`SpecialAttack_13_F33085FB4F8F0230AF14D2A8301C2B10` _specialattack)) (break `/Game/Core/Characters/S_Stats` (`/Game/Characters/Pokemon/BP_PokemonData.CurrentStats` (`self.UserPokemon`))))
  (if (> (`KismetMathLibrary.RandomIntegerInRange` 0 100) _accuracy)
    (`KismetSystemLibrary.PrintString` null "Attack miss")
    (else
      (switch `/Game/Blueprints/Attacks/E_AttackTypes` _attacktype
        (:`NewEnumerator0`
          (bind _damage (`self.DamageCalculation` _attack (`.Defense_9_F239144542E443A5B8D98284EEDCBDEA` (break `/Game/Core/Characters/S_Stats` (`/Game/Characters/Pokemon/BP_PokemonData.CurrentStats` _target_2)))))
          (`/Game/Characters/Pokemon/BP_PokemonData.DealDamage` _target_2 _damage))
        (:`NewEnumerator1`
          (bind _damage_2 (`self.DamageCalculation` _specialattack (`.SpecialDefense_14_534C8DA64CC4B30700C133A16E66F3F8` (break `/Game/Core/Characters/S_Stats` (`/Game/Characters/Pokemon/BP_PokemonData.CurrentStats` _target)))))
          (`/Game/Characters/Pokemon/BP_PokemonData.DealDamage` _target _damage_2))))))

(fn `DamageCalculation`
  (params (UserAttack :type Integer) (TargetDefense :type Integer))
  (returns (Damage :type Integer))
  (locals (Level :type "Float (double-precision)" :default 100.0) (Targets :type "Float (double-precision)" :default 1.0) (Weather :type "Float (double-precision)" :default 1.0) (Critical :type "Float (double-precision)" :default 1.0) (Random :type "Float (double-precision)" :default 1.0) (STAB :type "Float (double-precision)" :default 1.0) (Type :type "Float (double-precision)" :default 1.0) (Burn :type "Float (double-precision)" :default 1.0) (Other :type "Float (double-precision)" :default 1.0) (RelevantUserAttack :type "Float (double-precision)") (RelevantTargetDefense :type "Float (double-precision)"))
  (set `local.RelevantUserAttack` (`KismetMathLibrary.Conv_IntToDouble` UserAttack))
  (set `local.RelevantTargetDefense` (`KismetMathLibrary.Conv_IntToDouble` TargetDefense))
  (return (`KismetMathLibrary.FTrunc` (* (+ (/ (`KismetMathLibrary.Conv_IntToDouble` (`KismetMathLibrary.FTrunc` (* (`KismetMathLibrary.Conv_IntToDouble` (`KismetMathLibrary.FTrunc` (* (`.Power_14_3B64F1C748BF697183A0BEB2A844192C` (break `/Game/Blueprints/Attacks/S_Attacks` (`self.Attack`))) (+ (/ (* 2 (`local.Level`)) 5.0) 2.0)))) (/ (`local.RelevantUserAttack`) (`local.RelevantTargetDefense`))))) 50.0) 2.0) (`local.Targets`) (`local.Weather`) (`local.Critical`) (`local.Random`) (`local.STAB`) (`local.Type`) (`local.Burn`) (`local.Other`)))))